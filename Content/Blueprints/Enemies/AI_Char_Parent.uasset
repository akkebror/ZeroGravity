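; Parent enemy AI character that locks onto a player movement or combat character seen by PawnSensing, then pursues and shoots it.
; Each tick it smoothly turns toward the target, chases, retreats or brakes by distance, and roughly matches the target's height.
; Velocity is interpolated down to reduce orbiting.
; Firing is enabled only in the middle range, with a Delay throttling aimed Projectile_parent spawns.
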(event OnSeePawn(PawnSensing)
  (params (Pawn :type Pawn%20Object%20Reference))
  (Utilities|FlowControl|Sequence
    (:then_0
      (bind _asbp_character_movement (Utilities|Casting|CastToBP_Character_Movement Pawn))
      (Variables|Default|SetTarget _asbp_character_movement))
    (:then_1
      (bind _asbp_character_combat (Utilities|Casting|CastToBP_Character_Combat Pawn))
      (Variables|Default|SetTarget _asbp_character_combat)))
  (Variables|Default|SetTargetFound true))

(event EventTick
  (params (DeltaSeconds :type Float%20%28single-precision%29))
  (if (Variables|Default|GetTargetFound)
    (CallFunction|Turn)
    (CallFunction|Moveto)
    (Utilities|Fire)))

(fn ConstructionScript)

(fn Turn
  (Transformation|SetActorRotation (Math|Interpolation|RInterpTo (Transformation|GetActorRotation) (Math|Rotator|FindLookatRotation (Transformation|GetActorLocation) (Transformation|GetActorLocation (Variables|Default|GetTarget))) (Utilities|Time|GetWorldDeltaSeconds) 8.0)))

(fn Moveto
  (bind _returnvalue (Transformation|GetActorLocation))
  (bind _target (Variables|Default|GetTarget))
  (bind _target_2 (Variables|Default|GetTarget))
  (bind _returnvalue_2 (Transformation|GetDistanceTo _target_2))
  (bind _returnvalue_3 (Transformation|GetActorLocation _target))
  (bind _returnvalue_4 (- (.z _returnvalue_3) (.z _returnvalue)))
  (Utilities|FlowControl|Sequence
    (:then_0
      ;[1 1 1] Check distance to palyer and decide if you should chase or escape or stand still and fire
      (if (< _returnvalue_2 (Variables|Default|GetMoveUpTo))
        (if (> _returnvalue_2 (Variables|Default|GetFallBackWhen))
          (CallFunction|StopMovement)
          (Variables|Default|SetCanFire true)
          (else
            (Variables|Default|SetCanFire false)
            (CallFunction|MoveAI -1.0)))
        (else
          (Variables|Default|SetCanFire false)
          (CallFunction|MoveAI 1.0))))
    (:then_1
      ;[1 1 1] Adjust in order to keep the AI in roughly the same height as the player
      (if (> (Math|Float|Absolute(Float) _returnvalue_4) 3e+02)
        (Pawn|Input|AddMovementInput (Transformation|GetActorUpVector) (select (< _returnvalue_4 0.0) -1.0 1.0) false)))))

(fn MoveAI
  (params (Direction :type Float%20%28single-precision%29))
  (bind _charactermovement (Variables|Character|GetCharacterMovement))
  ;[1 1 1] Move
  (Pawn|Input|AddMovementInput (Transformation|GetActorForwardVector) Direction false)
  ;;[1 1 1] Removes some of the collected velocity in order to make the AI movement less orbital.
  (Variables|/Script/Engine.MovementComponent|SetVelocity _charactermovement (Math|Interpolation|VInterpTo (Variables|/Script/Engine.MovementComponent|GetVelocity _charactermovement) "0, 0, 0" (Utilities|Time|GetWorldDeltaSeconds) 2.0)))

(fn StopMovement
  (bind _charactermovement (Variables|Character|GetCharacterMovement))
  (Variables|/Script/Engine.MovementComponent|SetVelocity _charactermovement (Math|Interpolation|VInterpTo (Variables|/Script/Engine.MovementComponent|GetVelocity _charactermovement) "0, 0, 0" (Utilities|Time|GetWorldDeltaSeconds) 3.0)))